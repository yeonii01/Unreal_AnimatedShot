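; Trap gimmick Blueprint that shows its charge through light and destroys itself once its activation effect finishes.
; Each tick, after the parent's logic, it scales spotlight intensity from CurrentCharge.
; ActivateTrap switches on the particle system, binds finish events on it and the Niagara effect, then calls the parent implementation.
; Whichever bound effect reports finishing first destroys the actor.
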(event Custom|CustomEvent
  (params (PSystem :type Particle%20System%20Component%20Object%20Reference))
  (Actor|DestroyActor))

(event Custom|CustomEvent_1
  (params (PSystem :type Niagara%20Component%20Object%20Reference))
  (Actor|DestroyActor))

(event EventBeginPlay)

(event Collision|EventActorBeginOverlap
  (params (OtherActor :type Actor%20Object%20Reference)))

(event EventTick
  (params (DeltaSeconds :type Float%20%28single-precision%29))
  (|CallParentFunction DeltaSeconds)
  (Rendering|Components|Light|SetIntensity (Variables|Default|GetSpotLight) (* (Variables|Default|GetCurrentCharge) 1e+04)))

(event EventActivateTrap
  (bind _particlesystem (Variables|Default|GetParticleSystem))
  (Components|Activation|SetActive _particlesystem true false)
  (EventDispatchers|BindEventtoOnSystemFinished (Variables|Default|GetNiagaraEffect) (delegate Custom|CustomEvent_1))
  (EventDispatchers|BindEventtoOnSystemFinished _particlesystem (delegate Custom|CustomEvent))
  (|CallParentFunction))

(fn ConstructionScript)
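; BP_Sword is a VFX actor that plays a repeating, staggered sequence of four effect components, N1 to N4.
; Tick drives a DoOnce gate that activates each component in turn with reset, separated by short delays.
; After a longer pause the gate resets, so the next tick restarts the sequence in an endless loop without a timer.
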(event EventBeginPlay)

(event Collision|EventActorBeginOverlap
  (params (OtherActor :type Actor%20Object%20Reference)))

(event EventTick
  (params (DeltaSeconds :type Float%20%28single-precision%29))
  (Utilities|FlowControl|DoOnce false :!label _label
    (:Completed
      (Components|Activation|Activate (Variables|Default|GetN1) true)
      (Utilities|FlowControl|Delay 0.2)
      (Components|Activation|Activate (Variables|Default|GetN2) true)
      (Utilities|FlowControl|Delay 0.2)
      (Components|Activation|Activate (Variables|Default|GetN3) true)
      (Utilities|FlowControl|Delay 0.2)
      (Components|Activation|Activate (Variables|Default|GetN4) true)
      (Utilities|FlowControl|Delay 4.0)
      (goto _label Reset))))

(fn ConstructionScript)
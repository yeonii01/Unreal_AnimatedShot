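; BP_Attacker is an actor in the AdvancedNiagaraVFX content whose mesh can dissolve and undissolve on demand.
; DissolveStart and UndissolveStart, both gated by the Disslove flag, each create a dynamic instance of the mesh's first material and restart their own timeline.
; Each timeline drives that material's DissolveAmount parameter every update.
; The graph holds no attack logic, and its construction script is empty.
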(event Custom|Dissolve%20Start
  (if (Variables|Default|GetDisslove)
    (bind _returnvalue (Rendering|Material|CreateDynamicMaterialInstance (Variables|Character|GetMesh) 0 0 "None" :!class /Script/Engine.PrimitiveComponent))
    (bind _value (Timeline|StartDissolve PlayFromStart)
      (:Update
        (Rendering|Material|SetScalarParameterValue _returnvalue "DissolveAmount" _value :!class /Script/Engine.MaterialInstanceDynamic)))))

(event Custom|Undissolve%20Start
  (if (Variables|Default|GetDisslove)
    (bind _returnvalue (Rendering|Material|CreateDynamicMaterialInstance (Variables|Character|GetMesh) 0 0 "None" :!class /Script/Engine.PrimitiveComponent))
    (bind _value (Timeline|StartUnDissolve PlayFromStart)
      (:Update
        (Rendering|Material|SetScalarParameterValue _returnvalue "DissolveAmount" _value :!class /Script/Engine.MaterialInstanceDynamic)))))

(event EventBeginPlay)

(event Collision|EventActorBeginOverlap
  (params (OtherActor :type Actor%20Object%20Reference)))

(event EventTick
  (params (DeltaSeconds :type Float%20%28single-precision%29)))

(fn ConstructionScript)
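; BP_Tranform is a VFX Blueprint that toggles a dissolve transformation between two meshes, Mesh and TranformMesh.
; BeginPlay creates a dynamic material instance for each mesh.
; DissolveStart branches on the Transform flag and plays one of two timeline pairs in parallel to drive each material's Amount parameter, flipping the flag when finished.
; UndissolveStart is an empty event, so DissolveStart handles both directions.
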(event Custom|Dissolve%20Start
  (if (Variables|Default|GetTransform?)
    (Utilities|FlowControl|Sequence
      (:then_0
        (bind _value (Timeline|Timeline_2 PlayFromStart)
          (:Update
            (Rendering|Material|SetScalarParameterValue (Variables|Default|GetDynamicMesh1) "Amount" _value :!class /Script/Engine.MaterialInstanceDynamic))
          (:Finished
            (Variables|Default|SetTransform? false))))
      (:then_1
        (bind _value_2 (Timeline|Timeline_3 PlayFromStart)
          (:Update
            (Rendering|Material|SetScalarParameterValue (Variables|Default|GetDynamicMesh2) "Amount" _value_2 :!class /Script/Engine.MaterialInstanceDynamic)))))
    (else
      (Utilities|FlowControl|Sequence
        (:then_0
          (bind _value_3 (Timeline|Timeline_0 PlayFromStart)
            (:Update
              (Rendering|Material|SetScalarParameterValue (Variables|Default|GetDynamicMesh1) "Amount" _value_3 :!class /Script/Engine.MaterialInstanceDynamic))
            (:Finished
              (Variables|Default|SetTransform? true))))
        (:then_1
          (bind _value_4 (Timeline|Timeline_1 PlayFromStart)
            (:Update
              (Rendering|Material|SetScalarParameterValue (Variables|Default|GetDynamicMesh2) "Amount" _value_4 :!class /Script/Engine.MaterialInstanceDynamic))))))))

(event Custom|Undissolve%20Start)

(event EventBeginPlay
  (bind _returnvalue (Rendering|Material|CreateDynamicMaterialInstance (Variables|Character|GetMesh) 0 0 "None" :!class /Script/Engine.PrimitiveComponent))
  (Variables|Default|SetDynamicMesh1 _returnvalue)
  (bind _returnvalue_2 (Rendering|Material|CreateDynamicMaterialInstance (Variables|Default|GetTranformMesh) 0 0 "None" :!class /Script/Engine.PrimitiveComponent))
  (Variables|Default|SetDynamicMesh2 _returnvalue_2))

(fn ConstructionScript)
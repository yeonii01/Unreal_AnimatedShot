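; Item data component that makes its owning actor a pickup for the inventory system.
; On Interact, it passes its item row name and quantity to the interactor's inventory component.
; If pickup succeeds and the row exists in DT_ItemData, it destroys the owning actor.
; FocusTarget returns an empty string, and the row's pickup sound is not used.
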(event EventBeginPlay)

(event EventTick
  (params (DeltaSeconds :type Float%20%28single-precision%29)))

(event EventInteract
  (params (Interactor :type AS%20Character%20Object%20Reference))
  (bind _bpc_inventory (Variables|/Game/MyCharacter/AS_Character.AS_Character_C|GetBPC_Inventory Interactor)
    (:then
      (bind _success (Default|Pickup _bpc_inventory (Utilities|Struct|BreakDataTableRowHandle (Variables|Default|GetItemID)) (Variables|Default|GetItemQuantity)))
      (if _success
        (bind _returnvalue (Utilities|GetDataTableRow "/Game/InventorySystem/ItemData/DT_ItemData.DT_ItemData" (Utilities|Struct|BreakDataTableRowHandle (Variables|Default|GetItemID)))
          (:then
            (Actor|DestroyActor (Components|GetOwner))))))
    (:else)))

(fn NewFunction)

(fn FocusTarget
  (return ""))
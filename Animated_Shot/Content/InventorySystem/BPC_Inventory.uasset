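; Inventory component that holds the owner's item slots and coin count and handles interaction with nearby actors.
; Once started, a looping timer sphere-traces around the owner, stores the InteractInterface target and updates the prompt widget; IA_Interact triggers it.
; Pickups fill matching stacks up to DT_ItemData limits, then empty slots, returning after one unit.
; Using an item decrements its slot and applies potion healing or scroll stat boosts to the player.
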(event Custom|CreateInteractMessage
  (bind _returnvalue (UserInterface|CreateWidget "/Game/InventorySystem/UI/WB_InteractMessage.WB_InteractMessage_C"))
  (bind _output_get (Variables|Default|SetWB_InteractMessage _returnvalue))
  (UserInterface|Viewport|AddtoViewport _output_get 0))

(event Custom|BeginInteraction
  (Utilities|Time|SetTimerbyEvent (delegate Custom|UpdateInteraction) 0.2 true))

(event Custom|UpdateInteraction
  (CallFunction|Interaction))

(event Input|EnhancedActionEvents|EnhancedInputActionIA_Interact
  (params (ActionValue :type Boolean) (ElapsedSeconds :type Float%20%28double-precision%29) (TriggeredSeconds :type Float%20%28double-precision%29) (InputAction :type Input%20Action%20Object%20Reference :default "/Game/MyCharacter/Input/Actions/IA_Interact.IA_Interact"))
  (:Started
    (bind _targetactor (Variables|Default|GetTargetActor)
      (:then
        (bind _asinteract_interface (Utilities|Casting|CastToInteractInterface _targetactor))
        (bind _asas_character (Utilities|Casting|CastToAS_Character (Components|GetOwner)))
        (Class|InteractInterface|Interact _asinteract_interface _asas_character))
      (:else))))

(event EventBeginPlay
  (Utilities|Array|Resize (Variables|Default|GetItemSlots) (Variables|Default|GetInventorySize)))

(fn PrintInventory
  (for (_array_element _array_index) (Variables|Default|GetItemSlots)
    (Development|PrintString (Utilities|String|Append (Utilities|String|ToString(Integer) _array_index) ":" (Utilities|String|ToString(Name) (.ItemID (Utilities|Struct|BreakS_ItemSlot _array_element))) ":" (Utilities|String|ToString(Integer) (.ItemQuantity (Utilities|Struct|BreakS_ItemSlot _array_element)))))))

(fn Interaction
  (bind _returnvalue (Components|GetOwner))
  (bind _returnvalue_2 (Transformation|GetActorLocation _returnvalue))
  (bind (_outhit _returnvalue_3) (Collision|SphereTraceByChannel _returnvalue_2 _returnvalue_2 (Variables|Default|GetInteractRadius) "TraceTypeQuery1" false (Utilities|Array|MakeArray (Components|GetOwner)) "None"))
  (if _returnvalue_3
    (bind _asinteract_interface (Utilities|Casting|CastToInteractInterface (.HitActor (Collision|BreakHitResult _outhit))))
    (if (!= (.HitActor (Collision|BreakHitResult _outhit)) (Variables|Default|GetTargetActor))
      (Variables|Default|SetTargetActor (.HitActor (Collision|BreakHitResult _outhit)))
      (bind _returnvalue_4 (Class|InteractInterface|OnFocusTarget _asinteract_interface))
      (Default|SetInteractMessage (Variables|Default|GetWB_InteractMessage) _returnvalue_4))
    (else
      (Variables|Default|SetTargetActor 0)
      (Default|SetInteractMessage (Variables|Default|GetWB_InteractMessage)))))

(fn Pickup
  (params (ItemID :type Name) (ItemQuantity :type Integer))
  (bind (_success _index) (CallFunction|AnySlotAvailable))
  (bind _output_get (LocalVariables|SetLocal_ItemQuantity ItemQuantity))
  (while (and (> _output_get 0) (not (LocalVariables|GetLocal_IsFull)))
    (bind (_success_2 _array_index) (CallFunction|FindSlot ItemID))
    (if _success_2
      (CallFunction|AddtoStack _array_index 1)
      (Math|Integer|DecrementInt (LocalVariables|GetLocal_ItemQuantity)
        (:%20%20
          (return true 0)))
      (elif _success
        (CallFunction|CreateNewStack ItemID 1 _index)
        (Math|Integer|DecrementInt (LocalVariables|GetLocal_ItemQuantity)
          (:%20%20
            (return true 0)))
        (else
          (LocalVariables|SetLocal_IsFull true)))))
  (return (not (LocalVariables|GetLocal_IsFull)) (LocalVariables|GetLocal_ItemQuantity)))

(fn FindSlot
  (params (ItemID :type Name))
  (for (_array_element _array_index) (Variables|Default|GetItemSlots)
    (if (and (== (.ItemID (Utilities|Struct|BreakS_ItemSlot _array_element)) ItemID) (< (.ItemQuantity (Utilities|Struct|BreakS_ItemSlot _array_element)) (CallFunction|GetMaxStackSize ItemID)))
      (return true _array_index)))
  (return false -1))

(fn GetMaxStackSize
  (params (ItemID :type Name))
  (bind _returnvalue (Utilities|GetDataTableRow "/Game/InventorySystem/ItemData/DT_ItemData.DT_ItemData" ItemID)
    (:then
      (return (.SlotQuantity (Utilities|Struct|BreakS_ItemData _returnvalue))))))

(fn AddtoStack
  (params (Index :type Integer) (ItemQuantity :type Integer))
  (bind _itemslots (Variables|Default|GetItemSlots))
  (bind _output (Utilities|Array|Get(acopy) _itemslots Index))
  (Utilities|Array|SetArrayElem (Variables|Default|GetItemSlots) 0 (Utilities|Struct|MakeS_ItemSlot (.itemid _output) (+ (.itemquantity _output) ItemQuantity))))

(fn AnySlotAvailable
  (for (_array_element _array_index) (Variables|Default|GetItemSlots)
    (if (== (.ItemQuantity (Utilities|Struct|BreakS_ItemSlot _array_element)) 0)
      (return true _array_index)))
  (return false -1))

(fn CreateNewStack
  (params (ItemID :type Name) (ItemQuantity :type Integer) (Index :type Integer))
  (Utilities|Array|SetArrayElem (Variables|Default|GetItemSlots) Index (Utilities|Struct|MakeS_ItemSlot ItemID ItemQuantity)))

(fn AddCoin
  (params (CoinValue :type Integer))
  (Variables|Default|SetCoin (+ CoinValue (Variables|Default|GetCoin))))

(fn PickupItem
  (params (Item :type AS%20Item%20Base%20Object%20Reference))
  (bind (_success _index) (CallFunction|AnySlotAvailable))
  (|CallParentFunction Item)
  (LocalVariables|SetItemID (.RowName (Utilities|Struct|BreakDataTableRowHandle (Variables|/Script/Animated_Shot.ASItemBase|GetItemDataHandle Item))))
  (bind _output_get (LocalVariables|SetLocal_ItemQuantity (Variables|/Script/Animated_Shot.ASItemBase|GetItemQuantity Item)))
  (while (and (> _output_get 0) (not (LocalVariables|GetLocal_IsFull)))
    (bind (_success_2 _array_index) (CallFunction|FindSlot (LocalVariables|GetItemID)))
    (if _success_2
      (CallFunction|AddtoStack _array_index 1)
      (Math|Integer|DecrementInt (LocalVariables|GetLocal_ItemQuantity)
        (:%20%20
          (return true)))
      (elif _success
        (CallFunction|CreateNewStack (LocalVariables|GetItemID) 1 _index)
        (Math|Integer|DecrementInt (LocalVariables|GetLocal_ItemQuantity)
          (:%20%20
            (return true)))
        (else
          (LocalVariables|SetLocal_IsFull true)))))
  (return (not (LocalVariables|GetLocal_IsFull))))

(fn UseItem
  (params (Indexs :type Integer))
  (bind _returnvalue (Game|GetPlayerCharacter 0))
  (bind _itemslots (Variables|Default|GetItemSlots))
  (bind _output (Utilities|Array|Get(acopy) _itemslots Indexs))
  (LocalVariables|SetLocalItemID (.itemid _output))
  (LocalVariables|SetLocalItemQuantity (.itemquantity _output))
  (if (== (LocalVariables|GetLocalItemQuantity) 1)
    (Utilities|Array|SetArrayElem (Variables|Default|GetItemSlots) Indexs (Utilities|Struct|MakeS_ItemSlot "None" 0))
    (else
      (CallFunction|UpdateStack Indexs 1)))
  (Utilities|IsValid (.PotionData (Utilities|Struct|BreakS_ItemData (CallFunction|GetItemData (LocalVariables|GetLocalItemID))))
    (:Is%20Valid
      (bind _returnvalue_2 (Class|ASPotionItemData|GetHealAmount (.PotionData (Utilities|Struct|BreakS_ItemData (CallFunction|GetItemData (LocalVariables|GetLocalItemID))))))
      (bind _asascharacter_player (Utilities|Casting|CastToASCharacterPlayer _returnvalue))
      (Class|ASCharacterStatComponent|HealHp (Variables|/Script/Animated_Shot.ASCharacterBase|GetStat _asascharacter_player) _returnvalue_2))
    (:Is%20Not%20Valid
      (Utilities|IsValid (.ScrollData (Utilities|Struct|BreakS_ItemData (CallFunction|GetItemData (LocalVariables|GetLocalItemID))))
        (:Is%20Valid
          (bind _returnvalue_3 (Class|ASScrollItemData|GetBaseStat (.ScrollData (Utilities|Struct|BreakS_ItemData (CallFunction|GetItemData (LocalVariables|GetLocalItemID))))))
          (bind _asascharacter_player_2 (Utilities|Casting|CastToASCharacterPlayer _returnvalue))
          (Class|ASCharacterStatComponent|AddBaseStat (Variables|/Script/Animated_Shot.ASCharacterBase|GetStat _asascharacter_player_2) _returnvalue_3))))))

(fn UpdateStack
  (params (Indexes :type Integer) (Quantityis :type Integer))
  (bind _itemslots (Variables|Default|GetItemSlots))
  (bind _output (Utilities|Array|Get(acopy) _itemslots Indexes))
  (Utilities|Struct|SetmembersinS_ItemSlot _output (- (.ItemQuantity (Utilities|Struct|BreakS_ItemSlot _output)) Quantityis)))

(fn GetItemData
  (params (RowName :type Name))
  (bind _returnvalue (Utilities|GetDataTableRow "/Game/InventorySystem/ItemData/DT_ItemData.DT_ItemData" RowName)
    (:then
      (return _returnvalue))))